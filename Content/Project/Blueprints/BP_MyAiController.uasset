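; AI controller that runs the BT_MyCharacter behavior tree on the BB_MyCharacter blackboard and feeds it perception results.
; On each perception update, every updated actor's first stimulus sets bSearch to whether it was successfully sensed and prints that value.
; Actors that cast to BP_MyCharacter are stored as TargetPlayer, even when sensing failed.
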(event OnPerceptionUpdated(AIPerception)
  (params (UpdatedActors :type Array%20of%20Actor%20Object%20References))
  (for _array_element UpdatedActors
    (bind _info (Class|AIPerceptionComponent|GetActorsPerception (Variables|Default|GetAIPerception) _array_element))
    (Development|PrintString (Utilities|String|ToString(Boolean) (.bSuccessfullySensed (Utilities|Struct|BreakAIStimulus (Utilities|Array|Get(acopy) (.LastSensedStimuli (Utilities|Struct|BreakActorPerceptionBlueprintInfo _info)))))))
    (AI|Components|Blackboard|SetValueasBool (AI|GetBlackboard 0) (Utilities|Name|MakeLiteralName "bSearch") (.bSuccessfullySensed (Utilities|Struct|BreakAIStimulus (Utilities|Array|Get(acopy) (.LastSensedStimuli (Utilities|Struct|BreakActorPerceptionBlueprintInfo _info))))))
    (bind _asbp_my_character (Utilities|Casting|CastToBP_MyCharacter _array_element))
    (AI|Components|Blackboard|SetValueasObject (AI|GetBlackboard 0) (Utilities|Name|MakeLiteralName "TargetPlayer") _asbp_my_character)))

(event EventBeginPlay
  (Class|AIController|UseBlackboard "/Game/Project/Blueprints/BB_MyCharacter.BB_MyCharacter")
  (AI|RunBehaviorTree "/Game/Project/Blueprints/BT_MyCharacter.BT_MyCharacter"))

(fn ConstructionScript)