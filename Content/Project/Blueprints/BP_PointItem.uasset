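; BP_PointItem is a collectible that awards points when an actor overlaps its Box.
; On overlap it messages that actor with its name and Point value, plays a sound, and destroys itself.
; The construction script loads Point and the mesh material from the DT_PointItem row named by PointItemDataName.
; From BeginPlay, two timelines animate STMBox, spinning its yaw and shifting its relative X location.
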(event OnComponentBeginOverlap(Box)
  (params (OverlappedComponent :type Primitive%20Component%20Object%20Reference) (OtherActor :type Actor%20Object%20Reference) (OtherComp :type Primitive%20Component%20Object%20Reference) (OtherBodyIndex :type Integer) (bFromSweep :type Boolean) (SweepResult :type Hit%20Result%20Structure%20%28by%20ref%29))
  (Class|BPIMyCharacter|CharacterHitAction(Message) OtherActor (Utilities|GetDisplayName self) (Variables|Default|GetPoint))
  (Audio|PlaySoundatLocation "/Game/Project/Assets/game_item/Pick_Up/Ashorttactilesou1.Ashorttactilesou1" (Transformation|GetActorLocation) "0, 0, 0" 1.0 1.0 0.0 0 0 0 0)
  (Actor|DestroyActor))

(event EventBeginPlay
  (Utilities|FlowControl|Sequence
    (:then_0
      (bind _rotate (Timeline|Rotate PlayFromStart)
        (:Update
          (if (< (Variables|Default|GetActorRotation) 3.6e+02)
            (Variables|Default|SetActorRotation _rotate)
            (else
              (Variables|Default|SetActorRotation 0.0)))
          (Transformation|SetRelativeRotation (Variables|Default|GetSTM_Box) (Math|Rotator|MakeRotator 0.0 0.0 (Variables|Default|GetActorRotation)) false false))))
    (:then_1
      (bind _movingvalue (Timeline|Moving PlayFromStart)
        (:Update
          (Transformation|SetRelativeLocation (Variables|Default|GetSTM_Box) (Math|Vector|MakeVector _movingvalue 0.0 0.0) false false))))))

(fn ConstructionScript
  (bind _returnvalue (Utilities|GetDataTableRow "/Game/Project/Blueprints/DT_PointItem.DT_PointItem" (Variables|Default|GetPointItemDataName))
    (:then
      (Variables|Default|SetPoint (.Point (Utilities|Struct|BreakST_PointItem _returnvalue)))
      (Rendering|Material|SetMaterial (Variables|Default|GetSTM_Box) 0 (.MemberVar (Utilities|Struct|BreakST_PointItem _returnvalue))))))